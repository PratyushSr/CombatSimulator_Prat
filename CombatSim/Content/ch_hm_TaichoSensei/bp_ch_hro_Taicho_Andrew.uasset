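; Player hero Taicho, handling camera-relative movement, sprint, jump, combo melee, crystal carving and caravan interaction.
; Mouse buttons select montage arrays for timer-chained combos, while an immobilize flag gates movement and attacks.
; Gaining armor fades from first to third person by revealing the mesh and extending the spring arm.
; Entering the caravan swaps controller possession and hides the hero; a 15-second loop respawns a missing companion.
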(event Custom|stop_animation
  ;[1 1 1] Locks Player Controls During Carving
  ;;[1 1 1] Carving Setup
  (bind _returnvalue (Animation|GetCurrentMontage :!class /Script/Engine.Character))
  (if (== _returnvalue 0)
    (Animation|StopAnimMontage _returnvalue)))

(event Custom|companion%20check
  ;[1 0.9732 0] spawn companion
  (bind _outactors (Actor|GetAllActorsOfClass 0))
  (if (Utilities|IsValid (Utilities|Array|Get(acopy) _outactors))
    (Utilities|FlowControl|Delay 15.0)
    (CallFunction|CompanionCheck)
    (else
      (Game|SpawnActorfromClass 0 (Transformation|GetActorTransform) "AdjustIfPossibleButDontSpawnIfColliding" 0 0)
      (Utilities|FlowControl|Delay 15.0)
      (CallFunction|CompanionCheck))))

(event Custom|addcombo
  ;[1 1 1] //Andrew/Chris - Adds Second Attack in Combo
  (bind _output_get (Variables|Default|Setattack_combo (+ (Variables|Default|Getattack_combo) 1)))
  (if (> _output_get (Utilities|Array|LastIndex (Variables|Default|Getcurrent%20combo)))
    (Variables|Default|Setattack_combo 0)
    (Variables|Default|Setattacking true)
    (Variables|Default|Setcan%20move false)
    (Utilities|FlowControl|Delay 1.5)
    (Variables|Default|Setattacking false)
    (Variables|Default|Setcan%20move true)
    (else
      (Utilities|FlowControl|Sequence
        (:then_0
          (Utilities|FlowControl|Delay (+ (Variables|Default|Getdelay) 0.015))
          (Variables|Default|Setattacking false))
        (:then_1
          (Utilities|FlowControl|RetriggerableDelay (+ (Variables|Default|Getdelay) 0.5))
          (Variables|Default|Setattack_combo 0))))))

(event Custom|imobolize
  ;[1 1 1] Variables for Mobilizing and Immobilizing Hero.
  (Variables|Default|Setimobolized true)
  (Variables|Default|Setcan%20move false)
  (Variables|/Script/Engine.CharacterMovementComponent|SetMaxWalkSpeed (Variables|Character|GetCharacterMovement) 0.0))

(event Custom|rotate%20character
  (Transformation|SetWorldRotation (Variables|Character|GetMesh) (Math|Rotator|MakeRotator 0.0 0.0 (+ (.yaw (Math|Rotator|MakeRotationfromAxes (Class|Pawn|GetLastMovementInputVector) "0, 0, 0" "0, 0, 0")) -9e+01)) false false))

(event Custom|get%20armor
  ;[1 1 1] FPS to 3PS Transition
  (bind _alpha (Timeline|fade_timer PlayFromStart)
    (:Update
      (Rendering|Material|SetScalarParameterValue (Variables|Default|Getfade_mat) "opacity" _alpha :!class /Script/Engine.MaterialInstanceDynamic))
    (:Finished
      (Utilities|FlowControl|DoOnce false
        (:Completed
          (Variables|Default|Sethas_armor true)
          (Development|SetHiddeninGame (Variables|Character|GetMesh) false true)
          (Development|SetHiddeninGame (Variables|Default|Getcrystal) true true)
          (Variables|/Script/Engine.SpringArmComponent|SetTargetArmLength (Variables|Default|GetSpringArm1) 465.0)
          (CallFunction|Unfade))))))

(event Custom|deposit
  (Variables|Default|Setcarrying false)
  (Development|SetHiddeninGame (Variables|Default|Getcrystal) true false))

(event Custom|mobolize%20player
  ;[1 1 1] Variables for Mobilizing and Immobilizing Hero.
  (Variables|Default|Setimobolized false)
  (Variables|Default|Setcan%20move true)
  (Variables|/Script/Engine.CharacterMovementComponent|SetMaxWalkSpeed (Variables|Character|GetCharacterMovement) 6e+02))

(event Custom|reset
  (Utilities|FlowControl|DoOnce false) ; enters at Reset
)

(event Custom|attack
  ;[1 1 1] //Andrew/Chris - ? - Enables Player to Attack. Also configures Player to attack while moving.
  (if (Variables|Default|Getcan%20move)
    (if (Variables|Default|Getattacking)
      (Utilities|FlowControl|DoOnce false
        (:Completed
          (Utilities|FlowControl|Delay (- (Utilities|Time|GetTimerRemainingTimebyHandle (Variables|Default|Getcurrent%20animation)) 0.0)))))
    (Variables|Default|Setattacking true)
    (bind _returnvalue (Animation|Montage|MontagePlay (Components|SkeletalMesh|GetAnimInstance (Variables|Character|GetMesh)) (Utilities|Array|Get(acopy) (Variables|Default|Getcurrent%20combo) (Variables|Default|Getattack_combo)) 1.0 "Duration" 0.0 true))
    (bind _returnvalue_2 (Utilities|Time|SetTimerbyFunctionName 0 "reset" _returnvalue))
    (Variables|Default|Setcurrent%20animation _returnvalue_2)
    (CallFunction|Reset)
    (Variables|Default|Setdelay _returnvalue)
    (if (not (Variables|Default|Getimobolized))
      (Variables|/Script/Engine.CharacterMovementComponent|SetMaxWalkSpeed (Variables|Character|GetCharacterMovement) 25.0)
      (CallFunction|Addcombo)
      (bind _outactors (Actor|GetAllActorsOfClass 0))
      (CallFunction|TakeDmg)
      (Utilities|FlowControl|RetriggerableDelay _returnvalue)
      (if (not (Variables|Default|Getimobolized))
        (Variables|/Script/Engine.CharacterMovementComponent|SetMaxWalkSpeed (Variables|Character|GetCharacterMovement) 6e+02)))))

(event Custom|unfade
  ;[1 1 1] FPS to 3PS Transition
  (bind _alpha (Timeline|fade_timer ReverseFromEnd)
    (:Update
      (Rendering|Material|SetScalarParameterValue (Variables|Default|Getfade_mat) "opacity" _alpha :!class /Script/Engine.MaterialInstanceDynamic))
    (:Finished
      (Utilities|FlowControl|DoOnce false
        (:Completed
          (Variables|Default|Sethas_armor true)
          (Development|SetHiddeninGame (Variables|Character|GetMesh) false true)
          (Development|SetHiddeninGame (Variables|Default|Getcrystal) true true)
          (Variables|/Script/Engine.SpringArmComponent|SetTargetArmLength (Variables|Default|GetSpringArm1) 465.0)
          (CallFunction|Unfade))))))

(event EventBeginPlay
  ;[1 1 1] set intial vars
  (if (Variables|Default|Gethas_armor)
    (Development|SetHiddeninGame (Variables|Character|GetMesh) false true)
    (Variables|/Script/Engine.SpringArmComponent|SetTargetArmLength (Variables|Default|GetSpringArm1) 465.0)
    (else
      (Development|SetHiddeninGame (Variables|Character|GetMesh) true true)
      (Variables|/Script/Engine.SpringArmComponent|SetTargetArmLength (Variables|Default|GetSpringArm1) 0.0)))
  (bind _outactors (Actor|GetAllActorsOfClass 0))
  (Variables|Default|Setcaravan 0 0)
  (Variables|Default|Setcaravan_controller_player (Pawn|GetController))
  (Variables|Default|Setcaravan_controller_ai (Pawn|GetController (.caravan (Variables|Default|Getcaravan))))
  (CallFunction|CompanionCheck))

(event EventPossessed
  (params (NewController :type Controller%20Object%20Reference))
  ;[1 1 1] //Andrew - Hides the Main Character and UnHides a New MainCharacter that is attached to the caravan.
  (Input|EnableInput (Game|GetPlayerController 0))
  (Rendering|SetActorHiddenInGame false))

(event Input|AxisEvents|InputAxismove_forward
  (params (AxisValue :type Float%20%28single-precision%29))
  ;[1 1 1] Player Movement (Andrew/Chris)?
  (if (not (Variables|Default|Getimobolized))
    (Pawn|Input|AddMovementInput (Math|Vector|GetForwardVector (Transformation|GetWorldRotation (Variables|Default|GetSpringArm1))) AxisValue false)
    (if (!= AxisValue 0.0)
      (CallFunction|RotateCharacter)
      ;;[1 1 1] Locks Player Controls During Carving
      (CallFunction|StopAnimation))))

(event Input|AxisEvents|InputAxismove_right
  (params (AxisValue :type Float%20%28single-precision%29))
  ;[1 1 1] Player Movement (Andrew/Chris)?
  (if (not (Variables|Default|Getimobolized))
    (Pawn|Input|AddMovementInput (Math|Vector|GetRightVector (Variables|Default|GetSpringArm1)) AxisValue false)
    (if (!= AxisValue 0.0)
      (CallFunction|RotateCharacter)
      ;;[1 1 1] Locks Player Controls During Carving
      (CallFunction|StopAnimation))))

(event Input|AxisEvents|InputAxismove_back
  (params (AxisValue :type Float%20%28single-precision%29))
  ;[1 1 1] Player Movement (Andrew/Chris)?
  (if (not (Variables|Default|Getimobolized))
    (Pawn|Input|AddMovementInput (Math|Vector|GetForwardVector (Transformation|GetWorldRotation (Variables|Default|GetSpringArm1))) AxisValue false)
    (if (!= AxisValue 0.0)
      (CallFunction|RotateCharacter)
      ;;[1 1 1] Locks Player Controls During Carving
      (CallFunction|StopAnimation))))

(event Input|AxisEvents|InputAxismove_left
  (params (AxisValue :type Float%20%28single-precision%29))
  ;[1 1 1] Player Movement (Andrew/Chris)?
  (if (not (Variables|Default|Getimobolized))
    (Pawn|Input|AddMovementInput (Math|Vector|GetRightVector (Variables|Default|GetSpringArm1)) AxisValue false)
    (if (!= AxisValue 0.0)
      (CallFunction|RotateCharacter)
      ;;[1 1 1] Locks Player Controls During Carving
      (CallFunction|StopAnimation))))

(event Input|MouseEvents|MouseX
  (params (AxisValue :type Float%20%28single-precision%29))
  (bind _springarm1 (Variables|Default|GetSpringArm1))
  (bind _returnvalue (Transformation|GetWorldRotation _springarm1))
  ;[1 1 1] Mouse Input Look?
  (Transformation|SetWorldRotation (Variables|Default|GetSpringArm1) (Math|Rotator|MakeRotator 0.0 (.pitch _returnvalue) (+ (* AxisValue 5.0) (.yaw _returnvalue))) false false))

(event Input|MouseEvents|MouseY
  (params (AxisValue :type Float%20%28single-precision%29))
  (bind _springarm1 (Variables|Default|GetSpringArm1))
  (bind _returnvalue (Transformation|GetWorldRotation _springarm1))
  ;[1 1 1] Mouse Input Look?
  (Transformation|SetWorldRotation (Variables|Default|GetSpringArm1) (Math|Rotator|MakeRotator 0.0 (Math|Float|Clamp(Float) (+ (.pitch _returnvalue) (* AxisValue 5.0)) -85.0 3e+01) (.yaw _returnvalue)) false false))

(event Input|MouseEvents|LeftMouseButton
  (params (Key :type Key%20Structure))
  ;[1 1 1] Attack Key-Binds: Left and Right Mouse Button
  (:Pressed
    (if (not (Variables|Default|Getimobolized))
      (Variables|Default|Setcurrent%20combo (Variables|Default|Getattacks_horizontal))
      (CallFunction|Attack))))

(event Input|KeyboardEvents|Q
  (params (Key :type Key%20Structure))
  ;[1 1 1] Begin Caravan
  (:Pressed
    (bind _outactors (Actor|GetAllActorsOfClass 0))
    (CallFunction|Follow)))

(event Input|KeyboardEvents|W
  (params (Key :type Key%20Structure))
  (:Pressed
    (Variables|Default|Setforward_pressed true))
  (:Released
    (Variables|Default|Setforward_pressed false)))

(event Input|MouseEvents|MiddleMouseButton
  (params (Key :type Key%20Structure))
  ;[1 1 1] Input - Binds Carve button to Middle Mouse Click. Allows Player 'toCarve.'
  (:Pressed
    (if (Variables|Default|Getcarrying)
      (if (Variables|Default|Getcaravan_ride_bool)
        (CallFunction|Deposit))
      (elif (Variables|Default|Getcarve_distance)
        (Transformation|SetActorRotation (Math|Rotator|MakeRotator 0.0 0.0 (.yaw (Math|Rotator|FindLookatRotation (Transformation|GetActorLocation) (Transformation|GetActorLocation (Variables|Default|Getcarvable))))))
        (Animation|Montage|PlayMontage (Variables|Character|GetMesh) "/Game/ch_hm_TaichoSensei/Animations/k_ch_hro_Taicho_move_crch_carve_00_Montage.k_ch_hro_Taicho_move_crch_carve_00_Montage"
          (:OnCompleted
            (Variables|Default|Setcarrying true)
            (Development|SetHiddeninGame (Variables|Default|Getcrystal) false false)))))))

(event Input|KeyboardEvents|LeftShift
  (params (Key :type Key%20Structure))
  (bind _charactermovement (Variables|Character|GetCharacterMovement))
  ;[1 1 1] sprint
  (:Pressed
    (if (not (Variables|Default|Getimobolized))
      (Variables|/Script/Engine.CharacterMovementComponent|SetMaxWalkSpeed _charactermovement 9e+02)))
  (:Released
    (if (not (Variables|Default|Getimobolized))
      (Variables|/Script/Engine.CharacterMovementComponent|SetMaxWalkSpeed _charactermovement 6e+02))))

(event Input|MouseEvents|RightMouseButton
  (params (Key :type Key%20Structure))
  ;[1 1 1] Attack Key-Binds: Left and Right Mouse Button
  (:Pressed
    (if (not (Variables|Default|Getimobolized))
      (if (Variables|Default|Getforward_pressed)
        (Variables|Default|Setcurrent%20combo (Variables|Default|Getattacks_t))
        (else
          (Variables|Default|Setcurrent%20combo (Variables|Default|Getattacks_vertical))))
      (CallFunction|Attack))))

(event Input|KeyboardEvents|SpaceBar
  (params (Key :type Key%20Structure))
  ;[1 1 1] // Chris/ Andrew?? - isJumping
  (:Pressed
    (Character|Jump)))

(event Input|KeyboardEvents|E
  (params (Key :type Key%20Structure))
  (bind _caravan (Variables|Default|Getcaravan))
  (bind _target (Variables|GetTarget _caravan))
  ;[1 1 1] //Andrew - Input 'E' - Player Caravan Animations. Player enters based on Proximity.
  (:Pressed
    (if (Variables|Default|Getcaravan_ride_bool)
      ;;[1 1 1] Changing Posession from Player to Caravan
      (Input|DisableInput (Game|GetPlayerController 0))
      (Pawn|Possess (Variables|Default|Getcaravan_controller_player) (.caravan (Variables|Default|Getcaravan)))
      (Pawn|Possess (Variables|Default|Getcaravan_controller_ai) self)
      (Transformation|SetActorLocation (Transformation|GetWorldLocation _target) false true)
      (Transformation|SetActorRotation (Transformation|GetWorldRotation _target))
      (Rendering|SetActorHiddenInGame true)
      (CallFunction|Unhide (.caravan (Variables|Default|Getcaravan))))))

(fn ConstructionScript
  (bind _returnvalue (Rendering|Material|CreateDynamicMaterialInstance "/Game/ch_hm_TaichoSensei/fade_camera.fade_camera" "None" :!class /Script/Engine.KismetMaterialLibrary))
  (bind _output_get (Variables|Default|Setfade_mat _returnvalue))
  (Rendering|Material|SetMaterial (Variables|Default|Getfade) 0 _output_get))