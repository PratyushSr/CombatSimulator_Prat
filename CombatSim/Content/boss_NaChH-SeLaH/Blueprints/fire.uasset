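; Fire projectile actor in the boss_NaChH-SeLaH folder that launches toward the player's position when it spawns.
; On BeginPlay it faces the player, then line traces along the cube's forward vector, ignoring the player, to set the end point.
; The Fire timeline lerps the actor from spawn to that hit location while scaling up the cube.
; Movement is unswept, and the file contains no damage or destroy logic.
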(event EventBeginPlay
  (bind _returnvalue (Transformation|GetActorLocation))
  (Variables|Default|Setstart (Transformation|GetActorLocation))
  (Transformation|SetActorRotation (Math|Rotator|FindLookatRotation (Variables|Default|Getstart) (Transformation|GetActorLocation (Game|GetPlayerCharacter 0))))
  (bind _outhit (Collision|LineTraceByChannel _returnvalue (+ _returnvalue (* (Math|Vector|GetForwardVector (Variables|Default|GetCube)) 3.5e+03)) "TraceTypeQuery1" false (Utilities|Array|MakeArray (Game|GetPlayerCharacter 0)) "None"))
  (Variables|Default|Setend (.location _outhit))
  (bind _newtrack_0 (Timeline|fire PlayFromStart)
    (:Update
      (Transformation|SetActorLocation (Math|Vector|Lerp(Vector) (Variables|Default|Getstart) (Variables|Default|Getend) _newtrack_0) false false)
      (Transformation|SetWorldScale3D (Variables|Default|GetCube) (* "1.000000,1.000000,1.000000" (Math|Float|Lerp 0.2 3.0 _newtrack_0))))))

(fn ConstructionScript)