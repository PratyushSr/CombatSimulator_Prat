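; Boss carvable actor that marks itself as the target the Taicho Andrew hero can carve while in range.
; Capsule begin overlap with the player character sets the hero's CarveDistance flag and stores this actor in its Carvable reference.
; End overlap clears both, leaving any carving logic outside this Blueprint.
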(event OnComponentBeginOverlap(Capsule)
  (params (OverlappedComponent :type Primitive%20Component%20Object%20Reference) (OtherActor :type Actor%20Object%20Reference) (OtherComp :type Primitive%20Component%20Object%20Reference) (OtherBodyIndex :type Integer) (bFromSweep :type Boolean) (SweepResult :type Hit%20Result%20Structure%20%28by%20ref%29))
  (bind _returnvalue (Game|GetPlayerCharacter 0))
  (if (== OtherActor _returnvalue)
    (bind _asbp_ch_hro_taicho_andrew (Utilities|Casting|CastTobp_ch_hro_Taicho_Andrew _returnvalue))
    (Variables|/Game/ch_hm_TaichoSensei/bp_ch_hro_Taicho_Andrew.bp_ch_hro_Taicho_Andrew_C|Setcarve_distance _asbp_ch_hro_taicho_andrew true)
    (Variables|/Game/ch_hm_TaichoSensei/bp_ch_hro_Taicho_Andrew.bp_ch_hro_Taicho_Andrew_C|Setcarvable _asbp_ch_hro_taicho_andrew self)))

(event OnComponentEndOverlap(Capsule)
  (params (OverlappedComponent :type Primitive%20Component%20Object%20Reference) (OtherActor :type Actor%20Object%20Reference) (OtherComp :type Primitive%20Component%20Object%20Reference) (OtherBodyIndex :type Integer))
  (bind _returnvalue (Game|GetPlayerCharacter 0))
  (if (== OtherActor _returnvalue)
    (bind _asbp_ch_hro_taicho_andrew (Utilities|Casting|CastTobp_ch_hro_Taicho_Andrew _returnvalue))
    (Variables|/Game/ch_hm_TaichoSensei/bp_ch_hro_Taicho_Andrew.bp_ch_hro_Taicho_Andrew_C|Setcarve_distance _asbp_ch_hro_taicho_andrew false)
    (Variables|/Game/ch_hm_TaichoSensei/bp_ch_hro_Taicho_Andrew.bp_ch_hro_Taicho_Andrew_C|Setcarvable _asbp_ch_hro_taicho_andrew 0)))

(fn ConstructionScript)